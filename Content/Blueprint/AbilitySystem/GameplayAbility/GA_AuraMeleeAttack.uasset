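; GA_AuraMeleeAttack is a spear melee attack gameplay ability that, so far, detects hits without applying damage.
; It sets the avatar's motion warp target to its combat target's location through the combat interface, then plays the attack montage.
; On the montage's melee gameplay event, it gathers live players around the combat socket and draws debug spheres on them.
; EndAbility sits inside that loop, so it runs only when someone is found.
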(event Ability|EventActivateAbility
  (bind _returnvalue (Ability|GetAvatarActorfromActorInfo))
  (bind _returnvalue_2 (Ability|GetAvatarActorfromActorInfo))
  (bind _returnvalue_3 (Class|EnemyInterface|GetCombatTarget(Message) _returnvalue))
  (bind _ascombat_interface (Utilities|Casting|CastToCombatInterface _returnvalue))
  (Class|CombatInterface|UpdateMotionWarpTarget _ascombat_interface (Transformation|GetActorLocation _returnvalue_3))
  (|PlayMontageandWaitProxy "None" "/Game/Assets/Enemies/Goblin/Animations/Spear/AM_SpearMeleeAttack.AM_SpearMeleeAttack" 1.0 "None" true 1.0 0.0
    (:then
      (Ability|Tasks|WaitGameplayEvent "(TagName=\"Event.Montage.Attack.Melee\")" 0
        (:EventReceived
          (bind _returnvalue_4 (Class|CombatInterface|GetCombatSocketLocation(Message) _returnvalue_2))
          (bind _outoverlappingactors (Class|AuraAbilitySystemLibrary|GetLivePlayerswithinRadius _returnvalue_2 (Utilities|Array|MakeArray _returnvalue_2) 4e+01 _returnvalue_4))
          (for _array_element _outoverlappingactors
            (Rendering|Debug|DrawDebugSphere (Transformation|GetActorLocation _array_element) 4e+01 12 "(R=0.102079,G=1.000000,B=0.000000,A=1.000000)" 3.0)
            (Ability|EndAbility)))))))

(event Ability|EventOnEndAbility
  (params (bWasCancelled :type Boolean)))