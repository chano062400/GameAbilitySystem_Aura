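; Enemy ranged attack gameplay ability that fires a projectile at the avatar's combat target.
; On activation it points the motion warp target at that target and plays a random montage from the avatar's tagged attack montages.
; The montage's gameplay event tag triggers the projectile spawn from its socket tag, aimed at the target's current location.
; The ability ends shortly after firing or when the montage completes, is interrupted or is cancelled.
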(event Ability|EventActivateAbility
  (bind _returnvalue (Ability|GetAvatarActorfromActorInfo))
  (bind _returnvalue_2 (Class|EnemyInterface|GetCombatTarget(Message) _returnvalue))
  (Variables|Default|SetCombatTarget _returnvalue_2)
  (bind _ascombat_interface (Utilities|Casting|CastToCombatInterface _returnvalue))
  (Class|CombatInterface|UpdateMotionWarpTarget _ascombat_interface (Transformation|GetActorLocation _returnvalue_2))
  (bind _returnvalue_3 (Class|CombatInterface|GetAttackMontage(Message) (Ability|GetAvatarActorfromActorInfo)))
  (if (> (Utilities|Array|Length _returnvalue_3) 0)
    (bind _output_get (Variables|Default|SetTagged%20Montage (Utilities|Array|Get(acopy) _returnvalue_3 (Math|Random|RandomIntegerinRange 0 (- (Utilities|Array|Length _returnvalue_3) 1)))))
    (|PlayMontageandWaitProxy "None" (.Montage (Utilities|Struct|BreakTaggedMontage _output_get)) 1.0 "None" true 1.0 0.0
      (:then
        (Ability|Tasks|WaitGameplayEvent (.MontageTag (Utilities|Struct|BreakTaggedMontage _output_get)) 0
          (:EventReceived
            (Class|AuraProjectileSpell|SpawnProjectile (Transformation|GetActorLocation (Variables|Default|GetCombatTarget)) (.SocketTag (Utilities|Struct|BreakTaggedMontage _output_get)))
            (Utilities|FlowControl|Delay 1.0)
            (Ability|EndAbility))))
      (:OnCompleted
        (Ability|EndAbility :!label _label))
      (:OnInterrupted
        (goto _label))
      (:OnCancelled
        (goto _label)))))

(event Ability|EventOnEndAbility
  (params (bWasCancelled :type Boolean)))