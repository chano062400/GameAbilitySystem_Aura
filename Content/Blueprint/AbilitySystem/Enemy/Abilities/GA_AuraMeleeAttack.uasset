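; Enemy melee attack gameplay ability that plays a random attack montage and damages nearby hostile players.
; On activation it sets the motion warp target to the combat target's location, then waits for the montage's tagged gameplay event.
; That event triggers a small radius query at the matching combat socket, damaging non-friends with blood effects and an impact sound on hit.
; The ability ends after the hit check or when the montage finishes.
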(event Ability|EventActivateAbility
  (bind _returnvalue (Ability|GetAvatarActorfromActorInfo))
  (bind _returnvalue_2 (Ability|GetAvatarActorfromActorInfo))
  (Variables|Default|SetHasHitTarget false)
  (bind _returnvalue_3 (Class|EnemyInterface|GetCombatTarget(Message) _returnvalue))
  (bind _ascombat_interface (Utilities|Casting|CastToCombatInterface _returnvalue))
  (Class|CombatInterface|UpdateMotionWarpTarget _ascombat_interface (Transformation|GetActorLocation _returnvalue_3))
  (bind _returnvalue_4 (Class|CombatInterface|GetAttackMontage(Message) (Ability|GetAvatarActorfromActorInfo)))
  (bind _output_get (Variables|Default|SetTagged%20Montage (Utilities|Array|Get(acopy) _returnvalue_4 (Math|Random|RandomIntegerinRange 0 (- (Utilities|Array|Length _returnvalue_4) 1)))))
  (if (> (Utilities|Array|Length _returnvalue_4) 0)
    (|PlayMontageandWaitProxy "None" (.Montage (Utilities|Struct|BreakTaggedMontage _output_get)) 1.0 "None" false 1.0 0.0
      (:then
        (Ability|Tasks|WaitGameplayEvent (.MontageTag (Utilities|Struct|BreakTaggedMontage _output_get)) 0
          (:EventReceived
            (bind _returnvalue_5 (Class|CombatInterface|GetCombatSocketLocation(Message) _returnvalue_2 (.MontageTag (Utilities|Struct|BreakTaggedMontage _output_get))))
            (Variables|Default|SetCombatSocketLocation _returnvalue_5)
            (bind _outoverlappingactors (Class|AuraAbilitySystemLibrary|GetLivePlayerswithinRadius _returnvalue_2 (Utilities|Array|MakeArray _returnvalue_2) 4e+01 _returnvalue_5))
            (for _array_element _outoverlappingactors
              (if (not (Class|AuraAbilitySystemLibrary|IsFriend (Ability|GetAvatarActorfromActorInfo) _array_element))
                (Class|AuraDamageGameplayAbility|CauseDamage _array_element)
                (Variables|Default|SetHasHitTarget true)
                (bind _returnvalue_6 (Class|CombatInterface|GetBloodEffect(Message) _array_element))
                (Niagara|SpawnSystematLocation _returnvalue_6 (Variables|Default|GetCombatSocketLocation))))
            (if (Variables|Default|GetHasHitTarget)
              (Audio|PlaySoundatLocation (.impactsound (Variables|Default|GetTagged%20Montage)) (Variables|Default|GetCombatSocketLocation) "0, 0, 0" 1.0 1.0 0.0 0 0 0 0))
            (Ability|EndAbility))))
      (:OnCompleted
        (Ability|EndAbility :!label _label))
      (:OnInterrupted
        (goto _label))
      (:OnCancelled
        (goto _label)))
    (else
      (Ability|EndAbility))))

(event Ability|EventOnEndAbility
  (params (bWasCancelled :type Boolean)))