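; Electrocute gameplay ability: a channeled lightning beam at the target under the cursor that chains to additional targets.
; A montage event locks caster movement and starts ShockLoop cues, with per-target cue parameters stored for later removal.
; A looping timer commits cost and deals damage until cost fails or the first target dies.
; Input release, padded server-side to a minimum cast time, applies damage effects to enemy targets, then commits cooldown.
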(event Custom|DamageAndCost
  (bind _returnvalue (Ability|CommitAbilityCost false))
  (if _returnvalue
    (CallFunction|ApplyDamage)
    (else
      (GameplayCue|RemoveGameplayCueOnActor(Looping) (Variables|Default|GetCueTarget) "(TagName=\"GameplayCue.ShockLoop\")" (Variables|Default|GetFirstTargetCueParam))
      (CallFunction|ClearTimerandEndAbility))))

(event Ability|EventActivateAbility
  (bind _returnvalue (Ability|GetAvatarActorfromActorInfo))
  (if (Utilities|DoesObjectImplementInterface (Ability|GetAvatarActorfromActorInfo) "/Script/Aura.CombatInterface")
    (bind _datahandle (|TargetDataUnderMouse)
      (:ValidData
        (Class|AuraBeamSpell|StoreMouseDataInfo (Ability|TargetData|GetHitResultfromTargetData _datahandle))
        (Class|AuraBeamSpell|StoreOwnerPlayerController)
        (Utilities|FlowControl|Sequence
          (:then_0
            (Variables|/Script/Engine.PlayerController|SetbShowMouseCursor (Variables|Default|GetOwnerPlayerController) false)
            (bind _asbp_aura_character (Utilities|Casting|CastToBP_AuraCharacter _returnvalue))
            (Variables|Default|SetAura%20Character _asbp_aura_character)
            (Class|CombatInterface|UpdateMotionWarpTarget(Message) _returnvalue (Variables|Default|GetMouseHitLocation))
            (GameplayCue|ExecuteGameplayCue :GameplayCueTag "(TagName=\"GameplayCue.ShockBurst\")")
            (|PlayMontageandWaitProxy "None" (Variables|Default|GetElectrocute%20Montage) 1.0 "None" false 1.0 0.0
              (:then
                (Ability|Tasks|WaitGameplayEvent "(TagName=\"Event.Montage.Electrocute\")" 0 true
                  (:EventReceived
                    (Class|CombatInterface|SetinShockLoop(Message) (Ability|GetAvatarActorfromActorInfo) true)
                    (Pawn|Components|CharacterMovement|DisableMovement (Variables|/Script/Engine.Character|GetCharacterMovement (Variables|Default|GetAura%20Character)))
                    (Class|AuraBeamSpell|TraceFirstTarget (Variables|Default|GetMouseHitLocation))
                    (bind _returnvalue_2 (Class|CombatInterface|GetWeapon(Message) (Variables|Default|GetOwnerCharacter)))
                    ;[1 1 1] 첫번째 타겟 GameplayCue Parameter
                    (Variables|Default|SetFirstTargetCueParam (Ability|GameplayCue|MakeGameplayCueParameters :Location (Variables|Default|GetMouseHitLocation) :SourceObject (Variables|Default|GetMouseHitActor) :TargetAttachComponent _returnvalue_2))
                    ;[1 1 1] MouseHitActor가 Enemy인지 아닌지
                    (bind _output_get (Variables|Default|SetFirstTarget%20is%20Enemy? (Utilities|DoesObjectImplementInterface (Variables|Default|GetMouseHitActor) "/Script/Aura.CombatInterface")))
                    (if _output_get
                      ;[1 1 1] Cue Target이 Enemy라면
                      (bind _output_get_2 (Variables|Default|SetCueTarget (Variables|Default|GetMouseHitActor)))
                      (Class|CombatInterface|SetIsBeingShocked(Message) _output_get_2 true)
                      (GameplayCue|AddGameplayCueOnActor(Looping) (Variables|Default|GetCueTarget) "(TagName=\"GameplayCue.ShockLoop\")" (Variables|Default|GetFirstTargetCueParam))
                      (bind _outadditionaltargets (Class|AuraBeamSpell|StoreAdditionalTargets))
                      (bind _output_get_3 (Variables|Default|SetAdditional%20Targets _outadditionaltargets))
                      (for _array_element _output_get_3
                        (CallFunction|AddShockLoopCuetoAdditionalTarget _array_element))
                      (else
                        ;[1 1 1] Cue Target이 Enemy가 아니라면
                        (Variables|Default|SetCueTarget (Ability|GetAvatarActorfromActorInfo))
                        (GameplayCue|AddGameplayCueOnActor(Looping) (Variables|Default|GetCueTarget) "(TagName=\"GameplayCue.ShockLoop\")" (Variables|Default|GetFirstTargetCueParam))))
                    (bind _returnvalue_3 (Utilities|Time|SetTimerbyEvent (delegate Custom|DamageAndCost) (Variables|Default|GetDamageDeltaTime) true))
                    (Variables|Default|SetDamageAndCostTimer _returnvalue_3))))))
          (:then_1
            (bind _timeheld (Ability|Tasks|WaitInputRelease false)
              (:OnRelease
                (Variables|Default|SetTime%20Held _timeheld)
                (if (< (Variables|Default|GetTime%20Held) (Variables|Default|GetMinSpellTime))
                  (Ability|HasAuthority
                    (:True
                      (Utilities|FlowControl|Delay (- (Variables|Default|GetMinSpellTime) (Variables|Default|GetTime%20Held)))
                      (if (Variables|Default|GetFirstTarget%20is%20Enemy?) :!label _label
                        (Class|CombatInterface|SetIsBeingShocked(Message) (Variables|Default|GetMouseHitActor) false)
                        (GameplayCue|RemoveGameplayCueOnActor(Looping) (Variables|Default|GetMouseHitActor) "(TagName=\"GameplayCue.ShockLoop\")" (Variables|Default|GetFirstTargetCueParam))
                        (Ability|HasAuthority
                          (:True
                            (Class|AuraAbilitySystemLibrary|ApplyDamageEffect (Class|AuraDamageGameplayAbility|MakeDamageEffectParamsfromClassDefaults (Variables|Default|GetMouseHitActor))))
                          (:False
                            _))
                        (for _array_element_2 (Variables|Default|GetAdditional%20Targets)
                          (Class|CombatInterface|SetIsBeingShocked(Message) _array_element_2 false)
                          (if (.ReturnValue (Utilities|Map|Find (Variables|Default|GetAdditionalActorsToCueParams) _array_element_2))
                            (GameplayCue|RemoveGameplayCueOnActor(Looping) _array_element_2 "(TagName=\"GameplayCue.ShockLoop\")" (.Value (Utilities|Map|Find (Variables|Default|GetAdditionalActorsToCueParams) _array_element_2)))
                            (Ability|HasAuthority
                              (:True
                                (Class|AuraAbilitySystemLibrary|ApplyDamageEffect (Class|AuraDamageGameplayAbility|MakeDamageEffectParamsfromClassDefaults _array_element_2))))))
                        (else
                          (GameplayCue|RemoveGameplayCueOnActor(Looping) (Ability|GetAvatarActorfromActorInfo) "(TagName=\"GameplayCue.ShockLoop\")" (Variables|Default|GetFirstTargetCueParam))))
                      (CallFunction|ClearTimerandEndAbility))
                    (:False
                      (CallFunction|PreparetoEndAbility)))
                  (else
                    (goto _label)))))))))
    (else
      (Ability|EndAbility))))

(event EventFirstTargetDead
  (params (DeadActor :type Actor%20Object%20Reference))
  (GameplayCue|RemoveGameplayCueOnActor(Looping) DeadActor "(TagName=\"GameplayCue.ShockLoop\")" (Variables|Default|GetFirstTargetCueParam))
  (for _array_element (Variables|Default|GetAdditional%20Targets)
    (Class|CombatInterface|SetIsBeingShocked(Message) _array_element false)
    (if (.ReturnValue (Utilities|Map|Find (Variables|Default|GetAdditionalActorsToCueParams) _array_element))
      (GameplayCue|RemoveGameplayCueOnActor(Looping) _array_element "(TagName=\"GameplayCue.ShockLoop\")" (.Value (Utilities|Map|Find (Variables|Default|GetAdditionalActorsToCueParams) _array_element)))))
  (CallFunction|ClearTimerandEndAbility))

(event EventAdditionalTargetDead
  (params (DeadActor :type Actor%20Object%20Reference))
  (bind _additionalactorstocueparams (Variables|Default|GetAdditionalActorsToCueParams))
  (bind (_value _returnvalue) (Utilities|Map|Find _additionalactorstocueparams DeadActor))
  (if _returnvalue
    (GameplayCue|RemoveGameplayCueOnActor(Looping) DeadActor "(TagName=\"GameplayCue.ShockLoop\")" _value)
    (Utilities|Array|RemoveItem (Variables|Default|GetAdditional%20Targets) DeadActor)))

(fn AddShockLoopCuetoAdditionalTarget
  (params (Additional%20Target :type Actor%20Object%20Reference))
  (bind _output_get (LocalVariables|SetTargetActor Additional%20Target))
  (Class|CombatInterface|SetIsBeingShocked(Message) _output_get true)
  (Utilities|Map|Add (Variables|Default|GetAdditionalActorsToCueParams) (LocalVariables|GetTargetActor) (Ability|GameplayCue|MakeGameplayCueParameters :Location (Transformation|GetActorLocation (LocalVariables|GetTargetActor)) :SourceObject (LocalVariables|GetTargetActor) :TargetAttachComponent (Variables|/Script/Engine.Actor|GetRootComponent (Variables|Default|GetMouseHitActor))))
  (GameplayCue|AddGameplayCueOnActor(Looping) (LocalVariables|GetTargetActor) "(TagName=\"GameplayCue.ShockLoop\")" (Ability|GameplayCue|MakeGameplayCueParameters :Location (Transformation|GetActorLocation (LocalVariables|GetTargetActor)) :SourceObject (LocalVariables|GetTargetActor) :TargetAttachComponent (Variables|/Script/Engine.Actor|GetRootComponent (Variables|Default|GetMouseHitActor)))))

(fn PreparetoEndAbility
  (Variables|/Script/Engine.PlayerController|SetbShowMouseCursor (Variables|Default|GetOwnerPlayerController) true)
  (Class|CombatInterface|SetinShockLoop(Message) (Ability|GetAvatarActorfromActorInfo) false)
  (Pawn|Components|CharacterMovement|SetMovementMode (Variables|/Script/Engine.Character|GetCharacterMovement (Variables|Default|GetAura%20Character)) "MOVE_Walking" 0))

(fn ApplyDamage
  (Class|AuraDamageGameplayAbility|CauseDamage (Variables|Default|GetMouseHitActor))
  (for _array_element (Variables|Default|GetAdditional%20Targets)
    (Utilities|IsValid _array_element
      (:Is%20Valid
        (Class|AuraDamageGameplayAbility|CauseDamage _array_element)))))

(fn ClearTimerandEndAbility
  (Utilities|Time|ClearandInvalidateTimerbyHandle (Variables|Default|GetDamageAndCostTimer))
  (Utilities|Array|Clear (Variables|Default|GetAdditional%20Targets))
  (Utilities|Map|Clear (Variables|Default|GetAdditionalActorsToCueParams))
  (Variables|Default|SetMouseHitActor 0)
  (Variables|Default|SetFirstTarget%20is%20Enemy? false)
  (Variables|Default|SetTime%20Held 0.0)
  (CallFunction|PreparetoEndAbility)
  (Ability|CommitAbilityCooldown false)
  (Ability|EndAbility))