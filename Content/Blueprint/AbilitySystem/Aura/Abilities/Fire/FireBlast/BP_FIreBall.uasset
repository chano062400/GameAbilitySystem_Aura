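; Boomerang fireball actor for the FireBlast ability that flies out, returns to an actor and explodes.
; A travel timeline lerps it forward to an apex, then a return timeline homes on ReturnToActor's current location.
; Within ExplodeDistance it calls OnHit, applies radial damage effects to nearby live players except its owner, then destroys itself.
; Each target gets an upward-pitched knockback and a death impulse away from the blast.
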(event EventBeginPlay)

(event Collision|EventActorBeginOverlap
  (params (OtherActor :type Actor%20Object%20Reference)))

(event EventTick
  (params (DeltaSeconds :type Float%20%28single-precision%29)))

(event EventStartOutgoingTimeline
  (bind _returnvalue (Components|GetOwner))
  (bind _array (Utilities|Array|MakeArray _returnvalue))
  (Variables|Default|SetInitial%20Location (Transformation|GetActorLocation))
  (Variables|Default|SetApex%20Location (+ (Variables|Default|GetInitial%20Location) (* (Transformation|GetActorForwardVector) (Variables|Default|GetTravel%20Distance))))
  (bind _새_트랙_0 (Timeline|Travel%20Timeline Play)
    (:Update
      (Transformation|SetActorLocation (Math|Vector|Lerp(Vector) (Variables|Default|GetInitial%20Location) (Variables|Default|GetApex%20Location) _새_트랙_0) false false))
    (:Finished
      (bind _새_트랙_0_2 (Timeline|Return%20Timeline Play)
        (:Update
          (bind _returntoactor (Variables|Default|GetReturnToActor)
            (:then
              (Transformation|SetActorLocation (Math|Vector|Lerp(Vector) (Variables|Default|GetApex%20Location) (Transformation|GetActorLocation _returntoactor) _새_트랙_0_2) false false)
              (if (<= (Math|Vector|VectorLength (- (Transformation|GetActorLocation) (Transformation|GetActorLocation (Variables|Default|GetReturnToActor)))) (Variables|Default|GetExplodeDistance))
                (Class|AuraProjectile|OnHit)
                (Utilities|Array|Add _array self)
                (bind _outoverlappingactors (Class|AuraAbilitySystemLibrary|GetLivePlayerswithinRadius self _array (Variables|Default|GetRadialDamageOuterRadius) (Transformation|GetActorLocation)))
                (Variables|Default|SetOverlapping%20Actors _outoverlappingactors)
                (Class|AuraAbilitySystemLibrary|SetRaidalDamageEffectParams (Variables|Default|GetExplosionDamageEffectParams) true (Variables|Default|GetRadialDamageInnerRadius) (Variables|Default|GetRadialDamageOuterRadius) (Transformation|GetActorLocation))
                (for _array_element (Variables|Default|GetOverlapping%20Actors)
                  (Variables|Default|SetDirection (- (Transformation|GetActorLocation _array_element) (Transformation|GetActorLocation)))
                  (Class|AuraAbilitySystemLibrary|SetEffectParamsTargetASC (Variables|Default|GetExplosionDamageEffectParams) (Ability|GetAbilitySystemComponent _array_element))
                  (Class|AuraAbilitySystemLibrary|SetKnockbackDirection (Variables|Default|GetExplosionDamageEffectParams) (Math|Vector|GetForwardVector (Math|Rotator|MakeRotator (.roll (Math|Rotator|MakeRotfromX (Variables|Default|GetDirection))) 45.0 (.yaw (Math|Rotator|MakeRotfromX (Variables|Default|GetDirection))))) (Variables|Default|GetKnockbackMagnitude))
                  (Class|AuraAbilitySystemLibrary|SetDeathImpulseDirection (Variables|Default|GetExplosionDamageEffectParams) (Variables|Default|GetDirection) (Variables|Default|GetDeathImpulseMagnitude))
                  (Class|AuraAbilitySystemLibrary|ApplyDamageEffect (Variables|Default|GetExplosionDamageEffectParams)))
                (Actor|DestroyActor)))
            (:else)))))))

(fn ConstructionScript)