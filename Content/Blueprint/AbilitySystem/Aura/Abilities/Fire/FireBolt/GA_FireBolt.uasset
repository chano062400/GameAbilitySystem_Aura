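; GA_FireBolt is the Aura character's Fire Bolt gameplay ability, which casts projectiles toward the target under the mouse.
; After committing, it takes the hit location and actor from mouse target data and updates the character's motion warp target through CombatInterface.
; It plays the cast montage and, on its gameplay event, spawns projectiles from the weapon socket with an overridden pitch and the hit actor as homing target.
; The ability ends when the montage completes, blends out, or is interrupted or cancelled.
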(event Ability|EventActivateAbility
  (Ability|CommitAbility)
  (bind _datahandle (|TargetDataUnderMouse)
    (:ValidData
      (Variables|Default|SetProjectileTargetLocation (.Location (Collision|BreakHitResult (Ability|TargetData|GetHitResultfromTargetData _datahandle))))
      (Variables|Default|SetMouse%20Hit%20Actor (.HitActor (Collision|BreakHitResult (Ability|TargetData|GetHitResultfromTargetData _datahandle))))
      (bind _asbp_aura_character (Utilities|Casting|CastToBP_AuraCharacter (Ability|GetAvatarActorfromActorInfo)))
      (bind _ascombat_interface (Utilities|Casting|CastToCombatInterface _asbp_aura_character))
      (Class|CombatInterface|UpdateMotionWarpTarget _ascombat_interface (Variables|Default|GetProjectileTargetLocation))
      (|PlayMontageandWaitProxy "None" "/Game/Assets/Characters/Aura/Animations/Abilities/AM_Cast_FireBolt.AM_Cast_FireBolt" 1.0 "None" true 1.0 0.0
        (:then
          (Ability|Tasks|WaitGameplayEvent "(TagName=\"Event.Montage.FireBolt\")" 0
            (:EventReceived
              (Class|AuraFireBolt|SpawnProjectiles (Variables|Default|GetProjectileTargetLocation) (GameplayTags|MakeLiteralGameplayTag "(TagName=\"CombatSocket.Weapon\")") true 65.0 (Variables|Default|GetMouse%20Hit%20Actor)))))
        (:OnCompleted
          (Ability|EndAbility :!label _label))
        (:OnBlendOut
          (goto _label))
        (:OnInterrupted
          (goto _label))
        (:OnCancelled
          (goto _label))))))

(event Ability|EventOnEndAbility
  (params (bWasCancelled :type Boolean)))