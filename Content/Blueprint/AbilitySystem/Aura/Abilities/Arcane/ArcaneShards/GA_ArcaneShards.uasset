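; Arcane Shards gameplay ability that shows a magic circle and, on input release, casts a burst of shards at the spot under the mouse.
; It spawns a point collection there for level-scaled, randomly rotated ground points, then plays a motion-warped montage.
; A montage event commits cost and starts a looping timer that, per point, applies radial knockback damage and fires a GameplayCue.
; After the last shard it commits cooldown and ends.
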(event Custom|Spawn%20Arcane%20Shards
  (bind _returnvalue (Ability|GetAvatarActorfromActorInfo))
  (if (< (Variables|Default|GetCount) (Variables|Default|GetNumOfShards))
    (Variables|Default|SetArcane%20Shards%20Spawn%20Location (Transformation|GetWorldLocation (Utilities|Array|Get(acopy) (Variables|Default|GetGround%20Points) (Variables|Default|GetCount))))
    (bind _outoverlappingactors (Class|AuraAbilitySystemLibrary|GetLivePlayerswithinRadius _returnvalue (Utilities|Array|MakeArray _returnvalue) (Variables|Default|GetRadialDamageOuterRadius) (Variables|Default|GetArcane%20Shards%20Spawn%20Location)))
    (Variables|Default|SetOut%20Overlapping%20Actors _outoverlappingactors)
    (for _array_element (Variables|Default|GetOut%20Overlapping%20Actors)
      (Class|AuraAbilitySystemLibrary|ApplyDamageEffect (Class|AuraDamageGameplayAbility|MakeDamageEffectParamsfromClassDefaults _array_element (Variables|Default|GetArcane%20Shards%20Spawn%20Location) true (- (Transformation|GetActorLocation _array_element) (Variables|Default|GetArcane%20Shards%20Spawn%20Location)) true (- (Transformation|GetActorLocation _array_element) (Variables|Default|GetArcane%20Shards%20Spawn%20Location)) true 45.0)))
    (Math|Integer|IncrementInt (Variables|Default|GetCount)
      (:%20%20
        (Class|GameplayAbility|ExecuteGameplayCuewithParams "(TagName=\"GameplayCue.ArcaneShards\")" (Ability|GameplayCue|MakeGameplayCueParameters :Location (Variables|Default|GetArcane%20Shards%20Spawn%20Location)))))
    (else
      (Utilities|Time|ClearandInvalidateTimerbyHandle (Variables|Default|GetSpawn%20Aracne%20Shards%20Timer))
      (Actor|DestroyActor (Variables|Default|GetPoint%20Collection))
      (Ability|CommitAbilityCooldown false)
      (Ability|EndAbility))))

(event Ability|EventActivateAbility
  (bind _returnvalue (Class|GameplayAbility|CheckAbilityCost))
  (if _returnvalue
    (Utilities|FlowControl|Sequence
      (:then_0
        (Class|PlayerInterface|ShowMagicCircle(Message) (Ability|GetAvatarActorfromActorInfo) 0))
      (:then_1
        (Ability|Tasks|WaitInputRelease false
          (:OnRelease
            (bind _datahandle (|TargetDataUnderMouse)
              (:ValidData
                (Variables|Default|SetMouse%20Hit%20Location (.Location (Collision|BreakHitResult (Ability|TargetData|GetHitResultfromTargetData _datahandle))))
                (bind _returnvalue_2 (Game|SpawnActorfromClass "/Game/Blueprint/Actor/BP_PointCollection.BP_PointCollection_C" (Math|Transform|MakeTransform (Variables|Default|GetMouse%20Hit%20Location) "0, 0, 0" "1.000000,1.000000,1.000000") "AlwaysSpawn" "MultiplyWithRoot" 0 0))
                (bind _output_get (Variables|Default|SetPoint%20Collection _returnvalue_2))
                (Variables|Default|SetNumOfShards (Math|Integer|Min(Integer) (Variables|Default|GetMaxNumOfShards) (Ability|GetAbilityLevel)))
                (Variables|Default|SetGround%20Points (Class|PointCollection|GetGroundPoints _output_get (Variables|Default|GetMouse%20Hit%20Location) (Variables|Default|GetNumOfShards) (Math|Random|RandomFloatinRange 0.0 3.6e+02)))
                (Class|CombatInterface|UpdateMotionWarpTarget(Message) (Ability|GetAvatarActorfromActorInfo) (Variables|Default|GetMouse%20Hit%20Location))
                (|PlayMontageandWaitProxy "None" "/Game/Assets/Characters/Aura/Animations/Abilities/AM_Cast_Arcane_Shards.AM_Cast_Arcane_Shards" 1.0 "None" false 1.0 0.0
                  (:then
                    (Ability|Tasks|WaitGameplayEvent "(TagName=\"Event.Montage.ArcaneShards\")" 0 true
                      (:then
                        ;[1 1 1] 타이머를 시작하고, 첫번째 Arcane Shard를 Spawn
                        (bind _returnvalue_3 (Utilities|Time|SetTimerbyEvent (delegate Custom|Spawn%20Arcane%20Shards) (Variables|Default|GetAracane%20Shards%20Spawn%20Delta%20Time) true))
                        (Variables|Default|SetSpawn%20Aracne%20Shards%20Timer _returnvalue_3)
                        (Class|PlayerInterface|HideMagicCircle(Message) (Ability|GetAvatarActorfromActorInfo))
                        (CallFunction|SpawnArcaneShards)
                        (Ability|CommitAbilityCost false)))))))))))))