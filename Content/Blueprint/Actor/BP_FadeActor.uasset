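; BP_FadeActor is a static mesh actor that can fade out and back in through FadeOut and Fadein events.
; The construction script caches original materials and builds dynamic instances from FadeMaterialInstances.
; Both events swap in these instances and play FadeTimeline forward or reversed to drive their "Fade" parameter.
; Fully faded out, the mesh ignores Visibility and GameTraceChannel2 traces; fully faded in, it restores original materials and blocking.
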(event EventBeginPlay)

(event EventFadeOut
  (CallFunction|SetMaterialtoDynamicMaterialInstance)
  (bind _fadeouttrack (Timeline|FadeTimeline PlayFromStart)
    (:Update
      (for _array_element (Variables|Default|GetDynamic%20Material%20Instances)
        (Rendering|Material|SetScalarParameterValue _array_element "Fade" _fadeouttrack :!class /Script/Engine.MaterialInstanceDynamic)))
    (:Finished
      ;[1 1 1] Fade In이 끝나고
      (if (>= _fadeouttrack 1.0)
        (for (_array_element_2 _array_index) (Variables|Default|GetOriginal%20Materials)
          (Rendering|Material|SetMaterial (Variables|Default|GetStaticMesh) _array_index _array_element_2)
          (Collision|SetCollisionResponsetoChannel (Variables|Default|GetStaticMesh) "ECC_Visibility" "ECR_Block")
          (Collision|SetCollisionResponsetoChannel (Variables|Default|GetStaticMesh) "ECC_GameTraceChannel2" "ECR_Block"))
        (else
          ;[1 1 1] Fade Out이 끝나고
          (if (<= _fadeouttrack 0.0)
            (Collision|SetCollisionResponsetoChannel (Variables|Default|GetStaticMesh) "ECC_Visibility" "ECR_Ignore")
            (Collision|SetCollisionResponsetoChannel (Variables|Default|GetStaticMesh) "ECC_GameTraceChannel2" "ECR_Ignore")))))))

(event EventFadein
  (CallFunction|SetMaterialtoDynamicMaterialInstance)
  (bind _fadeouttrack (Timeline|FadeTimeline Reverse)
    (:Update
      (for _array_element (Variables|Default|GetDynamic%20Material%20Instances)
        (Rendering|Material|SetScalarParameterValue _array_element "Fade" _fadeouttrack :!class /Script/Engine.MaterialInstanceDynamic)))
    (:Finished
      ;[1 1 1] Fade In이 끝나고
      (if (>= _fadeouttrack 1.0)
        (for (_array_element_2 _array_index) (Variables|Default|GetOriginal%20Materials)
          (Rendering|Material|SetMaterial (Variables|Default|GetStaticMesh) _array_index _array_element_2)
          (Collision|SetCollisionResponsetoChannel (Variables|Default|GetStaticMesh) "ECC_Visibility" "ECR_Block")
          (Collision|SetCollisionResponsetoChannel (Variables|Default|GetStaticMesh) "ECC_GameTraceChannel2" "ECR_Block"))
        (else
          ;[1 1 1] Fade Out이 끝나고
          (if (<= _fadeouttrack 0.0)
            (Collision|SetCollisionResponsetoChannel (Variables|Default|GetStaticMesh) "ECC_Visibility" "ECR_Ignore")
            (Collision|SetCollisionResponsetoChannel (Variables|Default|GetStaticMesh) "ECC_GameTraceChannel2" "ECR_Ignore")))))))

(fn ConstructionScript
  (Utilities|Array|Clear (Variables|Default|GetDynamic%20Material%20Instances))
  (Variables|Default|SetOriginal%20Materials (Rendering|Material|GetMaterials (Variables|Default|GetStaticMesh)))
  (for _array_element (Variables|Default|GetFadeMaterialInstances)
    (bind _returnvalue (Rendering|Material|CreateDynamicMaterialInstance _array_element "None" "None" :!class /Script/Engine.KismetMaterialLibrary))
    (Utilities|Array|AddUnique (Variables|Default|GetDynamic%20Material%20Instances) _returnvalue)))

(fn SetMaterialtoDynamicMaterialInstance
  (for (_array_element _array_index) (Variables|Default|GetDynamic%20Material%20Instances)
    (Rendering|Material|SetMaterial (Variables|Default|GetStaticMesh) _array_index _array_element)))