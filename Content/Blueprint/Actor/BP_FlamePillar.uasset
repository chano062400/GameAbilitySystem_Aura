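; BP_FlamePillar is an actor that makes its flame light flicker with randomly varied intensity.
; On BeginPlay it randomly picks one of two timelines, and each picks again when it finishes, looping indefinitely.
; Each timeline update multiplies the track value by DefaultIntensity and applies the result to FlameLight.
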(event Custom|Timeline2
  (bind _새_트랙_0 (Timeline|타임라인 Play)
    (:Update
      (CallFunction|SetLightIntensity _새_트랙_0))
    (:Finished
      (CallFunction|ChooseTimeline))))

(event Custom|Timeline1
  (bind _새_트랙_0 (Timeline|FlameIntensityTimeline Play)
    (:Update
      (CallFunction|SetLightIntensity _새_트랙_0))
    (:Finished
      (CallFunction|ChooseTimeline))))

(event EventBeginPlay
  (CallFunction|ChooseTimeline))

(fn ConstructionScript)

(fn SetLightIntensity
  (params (Intensity :type Float%20%28double-precision%29))
  (Rendering|Components|Light|SetIntensity (Variables|Default|GetFlame%20Light) (* Intensity (Variables|Default|GetDefault%20Intensity))))

(fn ChooseTimeline
  (switch int (Math|Random|RandomIntegerinRange 0 1)
    (:0
      (CallFunction|Timeline1))
    (:1
      (CallFunction|Timeline2))))