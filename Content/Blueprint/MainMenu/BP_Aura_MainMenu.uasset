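; BP_Aura_MainMenu is a main menu actor that opens the menu and animates its scene dressing.
; BeginPlay plays the menu music, adds WBP_MainMenu to the viewport and switches to UI-only input with a visible cursor.
; Tick bobs Fire around its starting location with a sine wave whose timer resets every 2π.
; It also rolls MagicCIrcle by a fixed frame-rate-dependent step, skipping both animations on reset frames.
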(event EventBeginPlay
  (bind _returnvalue (Game|GetPlayerController 0))
  (Variables|Default|SetFire%20Location (Transformation|GetWorldLocation (Variables|Default|GetFire)))
  (Audio|PlaySound2D "/Game/Assets/Sounds/Music/Music_MainMenu.Music_MainMenu" 1.0 1.0 0.0 0 0)
  (bind _returnvalue_2 (UserInterface|CreateWidget "/Game/Blueprint/UI/MainMenu/WBP_MainMenu.WBP_MainMenu_C"))
  (UserInterface|Viewport|AddtoViewport _returnvalue_2 0)
  (Input|SetInputModeUIOnly _returnvalue 0 "DoNotLock" false)
  (Variables|/Script/Engine.PlayerController|SetbShowMouseCursor _returnvalue true))

(event EventTick
  (params (DeltaSeconds :type Float%20%28single-precision%29))
  ;[1 1 1] Sin은 2파이마다 주기적이므로
  (bind _output_get (Variables|Default|SetTime (+ DeltaSeconds (Variables|Default|GetTime))))
  (if (> _output_get 6.28318)
    (Variables|Default|SetTime 0.0)
    (else
      (Transformation|SetWorldLocation (Variables|Default|GetFire) (+ (Variables|Default|GetFire%20Location) (Math|Vector|MakeVector 0.0 0.0 (* (Math|Trig|Sin(Radians) (Variables|Default|GetTime)) 5.0))) false false)
      (Transformation|AddLocalRotation (Variables|Default|GetMagic%20CIrcle) (Math|Rotator|MakeRotator -0.1 0.0 0.0) false false))))

(fn ConstructionScript)